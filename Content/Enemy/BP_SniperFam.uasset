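; BP_SniperFam is a sniper enemy that turns toward the player character and shoots projectiles at it.
; When PawnSensing sees a BP_ThirdPersonCharacter, the whole actor snaps to a look-at rotation toward it.
; If CanAttack is set, it spawns a BP_SniperProjectile at SpawnProjectileLocation, then a fixed delay of a few seconds gates the next shot.
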(event `self.ReceiveBeginPlay`
  (`parent.ReceiveBeginPlay`))

(event `self.PawnSensing.OnSeePawn`
  (params (Pawn :type "Pawn Object Reference"))
  (bind (_returnvalue_x _returnvalue_y _returnvalue_z) (`KismetMathLibrary.BreakVector` (`self.K2_GetActorLocation`)))
  (bind _asbp_third_person_character (cast `/Game/ThirdPerson/Blueprints/BP_ThirdPersonCharacter` Pawn))
  (bind (_returnvalue_roll _returnvalue_pitch _returnvalue_yaw) (`KismetMathLibrary.BreakRotator` (`KismetMathLibrary.FindRelativeLookAtRotation` (`KismetMathLibrary.Conv_VectorToTransform` (`KismetMathLibrary.MakeVector` _returnvalue_x _returnvalue_y _returnvalue_z)) (`self.K2_GetActorLocation` _asbp_third_person_character))))
  (`self.K2_SetActorRotation` (`KismetMathLibrary.MakeRotator` _returnvalue_roll _returnvalue_pitch _returnvalue_yaw))
  (if (`self.CanAttack?`)
    (`|SpawnActorFromClass` "/Game/Projectile/BP_SniperProjectile.BP_SniperProjectile_C" (`SceneComponent.K2_GetComponentToWorld` (`self.SpawnProjectileLocation`)) "Undefined" "MultiplyWithRoot" null null)
    (set `self.CanAttack?` false)
    (`KismetSystemLibrary.Delay` 3.0)
    (set `self.CanAttack?` true)))

(fn `UserConstructionScript`
  (`parent.UserConstructionScript`))