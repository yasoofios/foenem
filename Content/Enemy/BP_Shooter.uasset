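; Enemy shooter AI that holds a pistol in its right hand and wanders to random reachable points until it sees a pawn.
; The first sighting latches it into a combat loop that alternates a timed shooting stance with runs to random nearby points.
; Each stance spawns another BP_Pistol at the Shoot transform, while a Delay-driven recursive event keeps it rotated toward the player.
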(event `self.ReceiveBeginPlay`
  (`parent.ReceiveBeginPlay`)
  (bind _returnvalue (`|SpawnActorFromClass` "/Game/Weapons/BP_Pistol.BP_Pistol_C" (`SceneComponent.GetSocketTransform` (`self.Mesh`) "RightHandSocket" "RTS_World") "Undefined" "MultiplyWithRoot" null null))
  (`self.K2_AttachToComponent` _returnvalue (`self.Mesh`) "RightHandSocket" "SnapToTarget" "SnapToTarget" "SnapToTarget" true)
  (bind _asbp_third_person_character (cast `/Game/ThirdPerson/Blueprints/BP_ThirdPersonCharacter` (`GameplayStatics.GetPlayerCharacter` 0)))
  (set `self.char_ref` _asbp_third_person_character)
  (`self.Walking`))

(event `Walking`
  (`|AIMoveTo` self (`NavigationSystemV1.K2_GetRandomReachablePointInRadius` (`self.K2_GetActorLocation`) 750.0 null null) null
    (:`OnSuccess`
      (if (not (`self.Spotted`))
        (`self.Walking`)))))

(event `self.PawnSensing.OnSeePawn`
  (params (Pawn :type "Pawn Object Reference"))
  (set `self.Spotted` true)
  (if (not (`self.shoot_player`))
    (set `CharacterMovementComponent.MaxWalkSpeed` 0.0 (`self.CharacterMovement`))
    (`self.Shooting`)))

(event `Shooting`
  (set `self.shoot_player` true)
  (`SkeletalMeshComponent.PlayAnimation` (`self.Mesh`) "/Game/Enemy/Shooter_assets/Shooting_Pistol.Shooting_Pistol" true)
  (set `self.face` true)
  (`self.Face Player`)
  (`|SpawnActorFromClass` "/Game/Weapons/BP_Pistol.BP_Pistol_C" (`SceneComponent.K2_GetComponentToWorld` (`self.Shoot`)) "Undefined" "MultiplyWithRoot" null null)
  (`KismetSystemLibrary.Delay` 3.0)
  (`SkeletalMeshComponent.PlayAnimation` (`self.Mesh`) "/Game/Enemy/Shooter_assets/Slow_Run.Slow_Run" true)
  (set `self.face` false)
  (`self.Run`))

(event `Run`
  (set `CharacterMovementComponent.MaxWalkSpeed` 250.0 (`self.CharacterMovement`))
  (`SkeletalMeshComponent.PlayAnimation` (`self.Mesh`) "/Game/Enemy/Shooter_assets/Slow_Run.Slow_Run" true)
  (`|AIMoveTo` self (`NavigationSystemV1.K2_GetRandomReachablePointInRadius` (`self.K2_GetActorLocation`) 500.0 null null) null
    (:`OnSuccess`
      (`self.Shooting`))))

(event `Face Player`
  (`self.K2_SetActorRotation` (`KismetMathLibrary.RInterpTo` (`self.K2_GetActorRotation`) (`KismetMathLibrary.FindLookAtRotation` (`self.K2_GetActorLocation`) (`self.K2_GetActorLocation` (`self.char_ref`))) (`GameplayStatics.GetWorldDeltaSeconds`)))
  (if (`self.face`)
    (`KismetSystemLibrary.Delay` 0.2)
    (`self.Face Player`)))

(fn `UserConstructionScript`
  (`parent.UserConstructionScript`))