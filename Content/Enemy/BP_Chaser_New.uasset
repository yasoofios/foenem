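; Zombie chaser enemy that patrols between two target points until it sees the player, then rushes in to punch, and is destroyed when its health runs out.
; PawnSensing triggers an AIMoveTo chase, and a delayed sphere overlap subtracts player health and triggers death at zero.
; After each punch, it widens its sight.
; A self-recalling delay loop started on BeginPlay continually rotates it toward the player, even during patrol.
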(event `self.ReceiveTick`
  (params (DeltaSeconds :type "Float (single-precision)"))
  (if (<= (`self.EnemyHealth`) 0)
    (`self.K2_DestroyActor`)))

(event `self.ReceiveBeginPlay`
  (`parent.ReceiveBeginPlay`)
  (bind _asbp_third_person_character (cast `/Game/ThirdPerson/Blueprints/BP_ThirdPersonCharacter` (`GameplayStatics.GetPlayerCharacter` 0)))
  (set `self.char_ref` _asbp_third_person_character)
  (`self.Face Player`)
  (`self.Walk`))

(event `Walk`
  ;[1 1 1] Walk
  (`SkeletalMeshComponent.PlayAnimation` (`self.Mesh`) "/Game/Enemy/Chaser_assests/Zombie_Walk.Zombie_Walk" true)
  (`|AIMoveTo` self (0.0 0.0 0.0) (`self.TargetPoint`)
    (:`OnSuccess`
      (`SkeletalMeshComponent.PlayAnimation` (`self.Mesh`) "/Game/Enemy/Chaser_assests/Zombie_Turn.Zombie_Turn" false)
      (`KismetSystemLibrary.Delay` 1.5)
      (`SkeletalMeshComponent.PlayAnimation` (`self.Mesh`) "/Game/Enemy/Chaser_assests/Zombie_Walk.Zombie_Walk" true)
      (`|AIMoveTo` self (0.0 0.0 0.0) (`self.TargetPoint2`)
        (:`OnSuccess`
          (`SkeletalMeshComponent.PlayAnimation` (`self.Mesh`) "/Game/Enemy/Chaser_assests/Zombie_Turn.Zombie_Turn" false)
          (`KismetSystemLibrary.Delay` 1.5)
          (`SkeletalMeshComponent.PlayAnimation` (`self.Mesh`) "/Game/Enemy/Chaser_assests/Zombie_Walk.Zombie_Walk" true)
          (`self.Walk`)
          (set `CharacterMovementComponent.MaxWalkSpeed` 100.0 (`self.CharacterMovement`))
          (set `self.Running` false))))))

(event `self.PawnSensing.OnSeePawn`
  (params (Pawn :type "Pawn Object Reference"))
  ;[1 1 1] Rush and attack player
  (`MovementComponent.StopMovementImmediately` (`self.CharacterMovement`))
  (if (not (`self.player_reached`))
    (if (not (`self.Running`))
      (`SkeletalMeshComponent.PlayAnimation` (`self.Mesh`) "/Game/Enemy/Chaser_assests/Zombie_Run.Zombie_Run" true)
      (set `self.Running` true))
    (`self.Rush Player` Pawn)))

(event `Rush Player`
  (params (Pawn :type "Pawn Object Reference"))
  (bind _pawnsensing (`self.PawnSensing`))
  ;[1 1 1] Rush and attack player
  (set `CharacterMovementComponent.MaxWalkSpeed` 500.0 (`self.CharacterMovement`))
  (`|AIMoveTo` self (0.0 0.0 0.0) Pawn
    (:`OnSuccess`
      (set `self.player_reached` true)
      (`SkeletalMeshComponent.PlayAnimation` (`self.Mesh`) "/Game/Enemy/Chaser_assests/Zombie_Punching.Zombie_Punching" false)
      (`KismetSystemLibrary.Delay` 0.85)
      (`GameplayStatics.PlaySound2D` "/Game/MilitaryWeapSilver/Sound/Knife/Wavs/Knife_ImpactSurface03.Knife_ImpactSurface03" 1.0 1.0 0.0 null null)
      (`self.Damage`)
      (`KismetSystemLibrary.Delay` 1.0)
      (set `self.player_reached` false)
      (`PawnSensingComponent.SetPeripheralVisionAngle` _pawnsensing 180.0)
      (set `PawnSensingComponent.SightRadius` 2000.0 _pawnsensing)
      (`SkeletalMeshComponent.PlayAnimation` (`self.Mesh`) "/Game/Enemy/Chaser_assests/Zombie_Run.Zombie_Run" true))))

(event `Damage`
  (bind _char_ref (`self.char_ref`))
  (bind _char_ref_2 (`self.char_ref`))
  ;[1 1 1] Damage player
  (bind _outactors (`KismetSystemLibrary.SphereOverlapActors` (`SceneComponent.K2_GetComponentLocation` (`self.Sphere`)) (`self.Sphere Radius`) (`|MakeArray` "ObjectTypeQuery3" :!type "EObjectTypeQuery Enum") "/Game/ThirdPerson/Blueprints/BP_ThirdPersonCharacter.BP_ThirdPersonCharacter_C" (`|MakeArray` self :!type "Actor Object Reference")))
  (for _ _outactors
    (set `/Game/ThirdPerson/Blueprints/BP_ThirdPersonCharacter.Health` (- (`/Game/ThirdPerson/Blueprints/BP_ThirdPersonCharacter.Health` _char_ref_2) 20) _char_ref_2)
    (if (<= (`/Game/ThirdPerson/Blueprints/BP_ThirdPersonCharacter.Health` _char_ref) 0)
      (set `/Game/ThirdPerson/Blueprints/BP_ThirdPersonCharacter.Health` 0 _char_ref)
      (`/Game/ThirdPerson/Blueprints/BP_ThirdPersonCharacter.PlayerDeath` _char_ref))))

(event `Face Player`
  ;[1 1 1] Face Player
  (if true
    _
    (else
      _))
  (`self.K2_SetActorRotation` (`KismetMathLibrary.RInterpTo` (`self.K2_GetActorRotation`) (`KismetMathLibrary.FindLookAtRotation` (`self.K2_GetActorLocation`) (`self.K2_GetActorLocation` (`self.char_ref`))) (`GameplayStatics.GetWorldDeltaSeconds`) 10.0))
  (`KismetSystemLibrary.Delay` 0.01)
  (`self.Face Player`))

(fn `UserConstructionScript`
  (`parent.UserConstructionScript`))