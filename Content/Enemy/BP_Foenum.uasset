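; BP_Foenum is a two-phase boss enemy that refills its health and plays a sound on first defeat, then is destroyed on the second.
; After a scream intro, a delay-driven loop continually turns it toward the player, with the Face flag having no effect.
; A recursive, animation-timed sequence alternates throwing with a crouched Exhausted window as its rock count runs out.
; ThrowRock is empty, and no damage handling appears here.
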(event `self.ReceiveTick`
  (params (DeltaSeconds :type "Float (single-precision)"))
  (if (<= (`self.Foenum_Health`) 0)
    (if (`self.Final_Phase`)
      (`self.K2_DestroyActor`)
      (else
        (set `self.Foenum_Health` 100)
        (set `self.Final_Phase` true)
        (`GameplayStatics.PlaySound2D` "/Engine/VREditor/Sounds/UI/Dockable_Window_Open.Dockable_Window_Open" 1.0 1.0 0.0 null null)))))

(event `self.ReceiveBeginPlay`
  (bind _asbp_third_person_character (cast `/Game/ThirdPerson/Blueprints/BP_ThirdPersonCharacter` (`GameplayStatics.GetPlayerCharacter` 0)))
  (set `self.char_ref` _asbp_third_person_character)
  (`SkeletalMeshComponent.PlayAnimation` (`self.Mesh`) "/Game/Enemy/BP_Foenum/Zombie_Scream.Zombie_Scream" false)
  (`KismetSystemLibrary.Delay` 2.78)
  (`SkeletalMeshComponent.PlayAnimation` (`self.Mesh`) "/Game/Enemy/BP_Foenum/Zombie_Idle.Zombie_Idle" true)
  (`self.Face Player`)
  (`self.Throw Sequence`))

(event `Face Player`
  ;[1 1 1] Face Player
  (if (`self.face`)
    _
    (else
      _))
  (`self.K2_SetActorRotation` (`KismetMathLibrary.RInterpTo` (`self.K2_GetActorRotation`) (`KismetMathLibrary.FindLookAtRotation` (`self.K2_GetActorLocation`) (`self.K2_GetActorLocation` (`self.char_ref`))) (`GameplayStatics.GetWorldDeltaSeconds`) 10.0))
  (`KismetSystemLibrary.Delay` 0.01)
  (`self.Face Player`))

(event `Throw Sequence`
  (if (`self.NotThrowing`)
    (set `self.NotThrowing` false)
    (`SkeletalMeshComponent.PlayAnimation` (`self.Mesh`) "/Game/Enemy/BP_Foenum/Throw_Object.Throw_Object" true))
  (`KismetSystemLibrary.Delay` 4.87)
  (set `self.Rocks` (- (`self.Rocks`) 1))
  (if (== (`self.Rocks`) 0)
    (set `self.face` false)
    (`SkeletalMeshComponent.PlayAnimation` (`self.Mesh`) "/Game/Enemy/BP_Foenum/Crouching.Crouching" false)
    (`KismetSystemLibrary.Delay` 4.07)
    (`SkeletalMeshComponent.PlayAnimation` (`self.Mesh`) "/Game/Enemy/BP_Foenum/Crouching_Idle.Crouching_Idle" false)
    (set `self.exhausted` true)
    (`KismetSystemLibrary.Delay` 4.0)
    (set `self.exhausted` false)
    (`SkeletalMeshComponent.PlayAnimation` (`self.Mesh`) "/Game/Enemy/BP_Foenum/Crouch_To_Stand.Crouch_To_Stand" false)
    (`KismetSystemLibrary.Delay` 3.33)
    (set `self.Rocks` 2)
    (set `self.NotThrowing` true)
    (`self.Throw Sequence`)
    (else
      (`self.Throw Sequence`))))

(event `Throw Rock`)

(fn `UserConstructionScript`)