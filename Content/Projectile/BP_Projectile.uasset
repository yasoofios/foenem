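; BP_Projectile is a projectile shared by player and enemies that deals damage on capsule overlap and expires after a timed lifetime.
; BeginPlay flags it as a player shot when its owner is the third-person character.
; Player shots damage BP_Enemy, award score and kill at zero health, and are destroyed only on lethal hits.
; Other shots damage the player character, destroying it at zero health, and are removed on that hit.
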(event `self.ReceiveBeginPlay`
  (cast `/Game/ThirdPerson/Blueprints/BP_ThirdPersonCharacter` (`self.GetOwner`))
  (set `self.playerShot` true))

(event `self.ReceiveTick`
  (params (DeltaSeconds :type "Float (single-precision)"))
  (bind _output_get (set `self.aliveTime` (- (`self.aliveTime`) DeltaSeconds)))
  (if (<= _output_get 0.0)
    (`self.K2_DestroyActor`)))

(event `self.Capsule.OnComponentBeginOverlap`
  (params (OverlappedComponent :type "PrimitiveComponent Object Reference") (OtherActor :type "Actor Object Reference") (OtherComp :type "PrimitiveComponent Object Reference") (OtherBodyIndex :type Integer) (bFromSweep :type Boolean) (SweepResult :type "HitResult Structure (by ref)"))
  (if (`self.playerShot`)
    (bind _asbp_enemy (cast `/Game/Enemy/BP_Enemy` OtherActor))
    (bind _returnvalue (- (`/Game/Enemy/BP_Enemy.EnemyHealth` _asbp_enemy) (`self.Damage`)))
    (if (<= _returnvalue 0)
      (bind _asbp_third_person_character (cast `/Game/ThirdPerson/Blueprints/BP_ThirdPersonCharacter` (`GameplayStatics.GetPlayerPawn` 0)))
      (set `/Game/ThirdPerson/Blueprints/BP_ThirdPersonCharacter.Score` (+ (`/Game/ThirdPerson/Blueprints/BP_ThirdPersonCharacter.Score` _asbp_third_person_character) (`/Game/Enemy/BP_Enemy.DeathScore` _asbp_enemy)) _asbp_third_person_character)
      (`/Game/Enemy/BP_Enemy.KillEnemy` _asbp_enemy)
      (`self.ProjectileDeletion`)
      (else
        (set `/Game/Enemy/BP_Enemy.EnemyHealth` _returnvalue _asbp_enemy)))
    (else
      (bind _asbp_third_person_character_2 (cast `/Game/ThirdPerson/Blueprints/BP_ThirdPersonCharacter` OtherActor))
      (bind _returnvalue_2 (- (`/Game/ThirdPerson/Blueprints/BP_ThirdPersonCharacter.Health` _asbp_third_person_character_2) (`self.Damage`)))
      (if (<= _returnvalue_2 0)
        (set `/Game/ThirdPerson/Blueprints/BP_ThirdPersonCharacter.Health` 0 _asbp_third_person_character_2)
        (`self.K2_DestroyActor` _asbp_third_person_character_2)
        (else
          (set `/Game/ThirdPerson/Blueprints/BP_ThirdPersonCharacter.Health` _returnvalue_2 _asbp_third_person_character_2)))
      (`self.ProjectileDeletion`))))

(event `ProjectileDeletion`
  (`self.K2_DestroyActor`))

(fn `UserConstructionScript`)