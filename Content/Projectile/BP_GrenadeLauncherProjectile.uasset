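; Grenade launcher projectile Blueprint that turns into an explosion when it is deleted.
; It overrides ProjectileDeletion to spawn BP_GrenadeLauncherExplosion at its own transform with the same owner, then calls the parent's deletion logic.
; Hit and overlap events on Blockcap and Overlapcap only print the other actor's name for debugging, so nothing connected here triggers deletion.
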(event `self.ProjectileDeletion`
  (`|SpawnActorFromClass` "/Game/Projectile/BP_GrenadeLauncherExplosion.BP_GrenadeLauncherExplosion_C" (`self.GetTransform`) "Undefined" "MultiplyWithRoot" (`self.GetOwner`) null)
  (`parent.ProjectileDeletion`))

(event `self.blockcap.OnComponentHit`
  (params (HitComponent :type "PrimitiveComponent Object Reference") (OtherActor :type "Actor Object Reference") (OtherComp :type "PrimitiveComponent Object Reference") (NormalImpulse :type "Vector Structure") (Hit :type "HitResult Structure (by ref)"))
  (`KismetSystemLibrary.PrintString` (`KismetSystemLibrary.GetDisplayName` OtherActor) true true (struct :`R` 1.0 :`B` 0.637006 :`A` 1.0)))

(event `self.overlapcap.OnComponentBeginOverlap`
  (params (OverlappedComponent :type "PrimitiveComponent Object Reference") (OtherActor :type "Actor Object Reference") (OtherComp :type "PrimitiveComponent Object Reference") (OtherBodyIndex :type Integer) (bFromSweep :type Boolean) (SweepResult :type "HitResult Structure (by ref)"))
  (`KismetSystemLibrary.PrintString` (`KismetSystemLibrary.GetDisplayName` OtherActor)))

(fn `UserConstructionScript`
  (`parent.UserConstructionScript`))