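; A level-exit collectible that saves the player's progress and opens the Overview level when the third-person character overlaps its capsule.
; It copies health, score, range, lore items and weapon state from the character into the game instance, then flags it as loaded and sets the next level number.
; GenerateWeaponString converts the weapon array into a list of names for storage in the game instance.
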(event `self.Capsule.OnComponentBeginOverlap`
  (params (OverlappedComponent :type "PrimitiveComponent Object Reference") (OtherActor :type "Actor Object Reference") (OtherComp :type "PrimitiveComponent Object Reference") (OtherBodyIndex :type Integer) (bFromSweep :type Boolean) (SweepResult :type "HitResult Structure (by ref)"))
  (bind _asbp_third_person_character (cast `/Game/ThirdPerson/Blueprints/BP_ThirdPersonCharacter` OtherActor))
  (bind _asbp_game_instance (cast `/Game/Levels/BP_GameInstance` (`GameplayStatics.GetGameInstance`)))
  (set `/Game/Levels/BP_GameInstance.PlayerHealth` (`/Game/ThirdPerson/Blueprints/BP_ThirdPersonCharacter.Health` _asbp_third_person_character) _asbp_game_instance)
  (set `/Game/Levels/BP_GameInstance.PlayerScore` (`/Game/ThirdPerson/Blueprints/BP_ThirdPersonCharacter.Score` _asbp_third_person_character) _asbp_game_instance)
  (set `/Game/Levels/BP_GameInstance.Range` (`/Game/ThirdPerson/Blueprints/BP_ThirdPersonCharacter.Range` _asbp_third_person_character) _asbp_game_instance)
  (set `/Game/Levels/BP_GameInstance.LoreItems` (`/Game/ThirdPerson/Blueprints/BP_ThirdPersonCharacter.LoreItems` _asbp_third_person_character) _asbp_game_instance)
  (set `/Game/Levels/BP_GameInstance.WeaponInd` (`/Game/ThirdPerson/Blueprints/BP_ThirdPersonCharacter.WeaponInd` _asbp_third_person_character) _asbp_game_instance)
  (bind _weaponnames (`self.GenerateWeaponString` (`/Game/ThirdPerson/Blueprints/BP_ThirdPersonCharacter.Weapons` _asbp_third_person_character)))
  (set `/Game/Levels/BP_GameInstance.PlayerWeapons` _weaponnames _asbp_game_instance)
  (set `/Game/Levels/BP_GameInstance.Loaded` true _asbp_game_instance)
  (set `/Game/Levels/BP_GameInstance.Level` 3 _asbp_game_instance)
  (`GameplayStatics.OpenLevelBySoftObjectPtr` "/Game/Levels/Overview.Overview"))

(fn `GenerateWeaponString`
  (params (Weapons :type "Array of /Game/Weapons/BP_Weapon Object Reference"))
  (returns (WeaponNames :type "Array of Name"))
  (bind _weaponstringarray (`self.WeaponStringArray`))
  (`KismetArrayLibrary.Array_Clear` (`self.WeaponStringArray`))
  (for _array_element Weapons
    (`KismetArrayLibrary.Array_Add` _weaponstringarray (`/Game/Weapons/BP_Weapon.Name` _array_element)))
  (return _weaponstringarray))

(fn `UserConstructionScript`
  (`parent.UserConstructionScript`))