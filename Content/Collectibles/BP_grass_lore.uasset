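; BP_grass_lore is a collectible lore pickup that triggers when BP_ThirdPersonCharacter overlaps its capsule.
; On overlap it adds its Lore to the character's LoreItems, pauses the game, and shows a WB_LoreOpen widget supplied with that lore.
; It then destroys itself and switches the player controller to UI-only input focused on the widget, with the mouse cursor visible.
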(event `self.Capsule.OnComponentBeginOverlap`
  (params (OverlappedComponent :type "PrimitiveComponent Object Reference") (OtherActor :type "Actor Object Reference") (OtherComp :type "PrimitiveComponent Object Reference") (OtherBodyIndex :type Integer) (bFromSweep :type Boolean) (SweepResult :type "HitResult Structure (by ref)"))
  (bind _lore (`self.Lore`))
  (bind _asbp_third_person_character (cast `/Game/ThirdPerson/Blueprints/BP_ThirdPersonCharacter` OtherActor))
  (`KismetArrayLibrary.Array_Add` (`/Game/ThirdPerson/Blueprints/BP_ThirdPersonCharacter.LoreItems` _asbp_third_person_character) _lore)
  (`GameplayStatics.SetGamePaused` true)
  (bind _returnvalue (`|CreateWidget` "/Game/ThirdPerson/Blueprints/WB_LoreOpen.WB_LoreOpen_C"))
  (`UserWidget.AddToViewport` _returnvalue 0)
  (`/Game/ThirdPerson/Blueprints/WB_LoreOpen.Supply Lore` _returnvalue _lore)
  (`self.K2_DestroyActor`)
  (bind _asplayer_controller (cast `PlayerController` (`Pawn.GetController` (`GameplayStatics.GetPlayerPawn` 0))))
  (`WidgetBlueprintLibrary.SetInputMode_UIOnlyEx` _asplayer_controller _returnvalue)
  (set `PlayerController.bShowMouseCursor` true _asplayer_controller))

(fn `UserConstructionScript`
  (`parent.UserConstructionScript`))