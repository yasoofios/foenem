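; BP_Pistol is a pistol weapon Blueprint that overrides the shoot and reload events of its weapon logic.
; InternalShoot, when ammo remains, spawns a projectile at the ShootingDir transform, decrements the bullet count, plays fire animation and sound, then clears Shooting.
; ReloadWeapon plays the reload animation and calls the parent reload; its sound call has no sound asset set.
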(event `self.InternalShoot`
  (bind _numbullets (`self.NumBullets`))
  (if (not (<= _numbullets 0))
    (`|SpawnActorFromClass` "/Game/Projectile/BP_PistolProjectile.BP_PistolProjectile_C" (`SceneComponent.K2_GetComponentToWorld` (`self.ShootingDir`)) "AlwaysSpawn" "MultiplyWithRoot" (`self.GetOwner`) null)
    (set `self.NumBullets` (- _numbullets 1))
    (`SkeletalMeshComponent.PlayAnimation` (`self.WeaponMesh`) "/Game/MilitaryWeapSilver/Weapons/Animations/Fire_Pistol_W.Fire_Pistol_W" false)
    (`GameplayStatics.PlaySoundAtLocation` "/Game/MilitaryWeapSilver/Sound/Pistol/Wavs/PistolA_Fire01.PistolA_Fire01" (`SceneComponent.K2_GetComponentLocation` (`self.DefaultSceneRoot`)) (struct) 1.0 1.0 0.0 null null null null)
    (set `self.Shooting` false)))

(event `self.ReloadWeapon`
  (`SkeletalMeshComponent.PlayAnimation` (`self.WeaponMesh`) "/Game/AnimStarterPack/Reload_Pistol.Reload_Pistol" false)
  (`GameplayStatics.PlaySoundAtLocation` null (`SceneComponent.K2_GetComponentLocation` (`self.DefaultSceneRoot`)) (struct) 1.0 1.0 0.0 null null null null)
  (`parent.ReloadWeapon`))

(fn `UserConstructionScript`
  (`parent.UserConstructionScript`))