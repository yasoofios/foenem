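; Machine gun weapon Blueprint that overrides shoot and reload events from its parent weapon class.
; Shooting, while bullets remain, spawns a machine gun projectile at the ShootingDir transform under the gun's owner, decrements the bullet count, and plays fire animation and sound.
; Reloading plays its own animation and sound, then hands the rest of the reload to the parent class.
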(event `self.ShootWeapon`
  (bind _numbullets (`self.NumBullets`))
  (if (not (<= _numbullets 0))
    (`|SpawnActorFromClass` "/Game/Projectile/BP_MachineGunProjectile.BP_MachineGunProjectile_C" (`SceneComponent.K2_GetComponentToWorld` (`self.ShootingDir`)) "AlwaysSpawn" "MultiplyWithRoot" (`self.GetOwner`) null)
    (set `self.NumBullets` (- _numbullets 1))
    (`SkeletalMeshComponent.PlayAnimation` (`self.WeaponMesh`) "/Game/AnimStarterPack/Fire_Rifle_Hip.Fire_Rifle_Hip" false)
    (`GameplayStatics.PlaySoundAtLocation` "/Game/MilitaryWeapSilver/Sound/Rifle/Wavs/RifleA_Fire01.RifleA_Fire01" (`SceneComponent.K2_GetComponentLocation` (`self.DefaultSceneRoot`)) (struct) 1.0 1.0 0.0 null null null null)))

(event `self.ReloadWeapon`
  (`SkeletalMeshComponent.PlayAnimation` (`self.WeaponMesh`) "/Game/AnimStarterPack/Prone_Reload_Rifle.Prone_Reload_Rifle" false)
  (`GameplayStatics.PlaySoundAtLocation` "/Game/MilitaryWeapSilver/Sound/Rifle/Wavs/Rifle_Reload01.Rifle_Reload01" (`SceneComponent.K2_GetComponentLocation` (`self.DefaultSceneRoot`)) (struct) 1.0 1.0 0.0 null null null null)
  (`parent.ReloadWeapon`))

(fn `UserConstructionScript`
  (`parent.UserConstructionScript`))