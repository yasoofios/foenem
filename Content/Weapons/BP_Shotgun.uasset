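; BP_Shotgun is a shotgun weapon that fires a spread of projectiles and overrides reload behavior from its parent.
; ShootWeapon, while bullets remain, spawns BP_ShotgunProjectile at four ShootingDir transforms, spends one bullet and plays the fire animation.
; Only the first projectile receives an Owner, and the fire sound node is unconnected.
; ReloadWeapon plays the reload animation and sound, then calls the parent's reload.
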(event `self.ShootWeapon`
  (bind _numbullets (`self.NumBullets`))
  (if (not (<= _numbullets 0))
    (`|SpawnActorFromClass` "/Game/Projectile/BP_ShotgunProjectile.BP_ShotgunProjectile_C" (`SceneComponent.K2_GetComponentToWorld` (`self.ShootingDir`)) "AlwaysSpawn" "MultiplyWithRoot" (`self.GetOwner`) null)
    (`|SpawnActorFromClass` "/Game/Projectile/BP_ShotgunProjectile.BP_ShotgunProjectile_C" (`SceneComponent.K2_GetComponentToWorld` (`self.ShootingDir1`)) "AlwaysSpawn" "MultiplyWithRoot" null null)
    (`|SpawnActorFromClass` "/Game/Projectile/BP_ShotgunProjectile.BP_ShotgunProjectile_C" (`SceneComponent.K2_GetComponentToWorld` (`self.ShootingDir2`)) "AlwaysSpawn" "MultiplyWithRoot" null null)
    (`|SpawnActorFromClass` "/Game/Projectile/BP_ShotgunProjectile.BP_ShotgunProjectile_C" (`SceneComponent.K2_GetComponentToWorld` (`self.ShootingDir3`)) "AlwaysSpawn" "MultiplyWithRoot" null null)
    (set `self.NumBullets` (- _numbullets 1))
    (`SkeletalMeshComponent.PlayAnimation` (`self.WeaponMesh`) "/Game/MilitaryWeapSilver/Weapons/Animations/Fire_Shotgun_W.Fire_Shotgun_W" false)))

(event `self.ReloadWeapon`
  (`SkeletalMeshComponent.PlayAnimation` (`self.WeaponMesh`) "/Game/AnimStarterPack/Reload_Shotgun_Hip.Reload_Shotgun_Hip" false)
  (`GameplayStatics.PlaySoundAtLocation` "/Game/MilitaryWeapSilver/Sound/Shotgun/Wavs/Shotgun_Reload03.Shotgun_Reload03" (`SceneComponent.K2_GetComponentLocation` (`self.DefaultSceneRoot`)) (struct) 1.0 1.0 0.0 null null null null)
  (`parent.ReloadWeapon`))

(fn `UserConstructionScript`
  (`parent.UserConstructionScript`))